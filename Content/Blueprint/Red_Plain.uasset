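; Red plain actor that shows and becomes solid only when the background colour differs from its own.
; BeginPlay caches the first Background_Sprite in the level and sets its own colour index to 1.
; Every Tick it compares the background's Colour to that index, hiding RedPlain and disabling its collision on a match, otherwise restoring visibility and query-and-physics collision.
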(event `self.ReceiveBeginPlay`
  (bind _outactors (`GameplayStatics.GetAllActorsOfClass` "/Game/Blueprint/Background_Sprite.Background_Sprite_C"))
  (set `self.BGColour` (`|GetArrayItem` _outactors))
  (set `self.MyColour` 1))

(event `self.ReceiveTick`
  (params (DeltaSeconds :type "Float (single-precision)"))
  (bind _red_plain (`self.Red_Plain`))
  (bind _red_plain_2 (`self.Red_Plain`))
  (`/Engine/EditorBlueprintResources/StandardMacros.CompareInt` (`/Game/Blueprint/Background_Sprite.Colour` (`self.BGColour`)) (`self.MyColour`)
    (:`>`
      (`PrimitiveComponent.SetCollisionEnabled` _red_plain_2 "QueryAndPhysics" :!label _label)
      (`SceneComponent.SetVisibility` _red_plain true false))
    (:`==`
      (`PrimitiveComponent.SetCollisionEnabled` _red_plain_2 "NoCollision")
      (`SceneComponent.SetVisibility` _red_plain false false))
    (:`<`
      (goto _label))))

(fn `UserConstructionScript`)