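; PinkBrick5 is a colour-keyed brick that disappears when the background colour matches its own colour index of 5.
; On BeginPlay it caches the first Background_Sprite actor found in the level.
; Every Tick it compares that actor's Colour to its own, hiding the sprite and disabling collision on a match, otherwise showing it with query and physics collision.
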(event `self.ReceiveBeginPlay`
  (bind _outactors (`GameplayStatics.GetAllActorsOfClass` "/Game/Blueprint/Background_Sprite.Background_Sprite_C"))
  (set `self.BGColour` (`|GetArrayItem` _outactors))
  (set `self.MyColour` 5))

(event `self.ReceiveTick`
  (params (DeltaSeconds :type "Float (single-precision)"))
  (bind _pinkbricksprite (`self.PinkBrickSprite`))
  (bind _pinkbricksprite_2 (`self.PinkBrickSprite`))
  (`/Engine/EditorBlueprintResources/StandardMacros.CompareInt` (`/Game/Blueprint/Background_Sprite.Colour` (`self.BGColour`)) (`self.MyColour`)
    (:`>`
      (`PrimitiveComponent.SetCollisionEnabled` _pinkbricksprite "QueryAndPhysics" :!label _label)
      (`SceneComponent.SetVisibility` _pinkbricksprite_2 true false))
    (:`==`
      (`PrimitiveComponent.SetCollisionEnabled` _pinkbricksprite "NoCollision")
      (`SceneComponent.SetVisibility` _pinkbricksprite_2 false false))
    (:`<`
      (goto _label))))

(fn `UserConstructionScript`)