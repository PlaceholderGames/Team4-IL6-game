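; BlueBrick4 is a brick actor that disappears when the background's colour matches its own colour index, 4.
; On BeginPlay it stores the first Background_Sprite actor it finds as its colour reference.
; Every Tick it compares the two colour values, hiding the sprite and disabling its collision on a match, and showing it with full collision otherwise.
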(event `self.ReceiveBeginPlay`
  (bind _outactors (`GameplayStatics.GetAllActorsOfClass` "/Game/Blueprint/Background_Sprite.Background_Sprite_C"))
  (set `self.BGColour` (`|GetArrayItem` _outactors))
  (set `self.MyColour` 4))

(event `self.ReceiveTick`
  (params (DeltaSeconds :type "Float (single-precision)"))
  (bind _bluebricksprite (`self.BlueBrickSprite`))
  (bind _bluebricksprite_2 (`self.BlueBrickSprite`))
  (`/Engine/EditorBlueprintResources/StandardMacros.CompareInt` (`/Game/Blueprint/Background_Sprite.Colour` (`self.BGColour`)) (`self.MyColour`)
    (:`>`
      (`PrimitiveComponent.SetCollisionEnabled` _bluebricksprite_2 "QueryAndPhysics" :!label _label)
      (`SceneComponent.SetVisibility` _bluebricksprite true false))
    (:`==`
      (`PrimitiveComponent.SetCollisionEnabled` _bluebricksprite_2 "NoCollision")
      (`SceneComponent.SetVisibility` _bluebricksprite false false))
    (:`<`
      (goto _label))))

(fn `UserConstructionScript`)