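; Light blue brick that disappears when the background takes on its colour.
; On BeginPlay it caches the first Background_Sprite actor and sets its own colour index to 6.
; Every Tick it compares the background's Colour to that index, hiding the brick and disabling collision on a match, otherwise keeping it visible and solid.
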(event `self.ReceiveBeginPlay`
  (bind _outactors (`GameplayStatics.GetAllActorsOfClass` "/Game/Blueprint/Background_Sprite.Background_Sprite_C"))
  (set `self.BGColour` (`|GetArrayItem` _outactors))
  (set `self.MyColour` 6))

(event `self.ReceiveTick`
  (params (DeltaSeconds :type "Float (single-precision)"))
  (bind _lightbluebrick (`self.LightBlueBrick`))
  (bind _lightbluebrick_2 (`self.LightBlueBrick`))
  (`/Engine/EditorBlueprintResources/StandardMacros.CompareInt` (`/Game/Blueprint/Background_Sprite.Colour` (`self.BGColour`)) (`self.MyColour`)
    (:`>`
      (`PrimitiveComponent.SetCollisionEnabled` _lightbluebrick "QueryAndPhysics" :!label _label)
      (`SceneComponent.SetVisibility` _lightbluebrick_2 true false))
    (:`==`
      (`PrimitiveComponent.SetCollisionEnabled` _lightbluebrick "NoCollision")
      (`SceneComponent.SetVisibility` _lightbluebrick_2 false false))
    (:`<`
      (goto _label))))

(fn `UserConstructionScript`)