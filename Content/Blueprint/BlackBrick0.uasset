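; BlackBrick0 is a brick actor that appears or disappears depending on the current background colour.
; On BeginPlay it caches the first Background_Sprite actor and sets its own colour index to 0.
; Every Tick it compares the background's Colour with that index, hiding the sprite and disabling its collision on a match, and showing it with query and physics collision otherwise.
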(event `self.ReceiveBeginPlay`
  (bind _outactors (`GameplayStatics.GetAllActorsOfClass` "/Game/Blueprint/Background_Sprite.Background_Sprite_C"))
  (set `self.BGColour` (`|GetArrayItem` _outactors))
  (set `self.MyColour` 0))

(event `self.ReceiveTick`
  (params (DeltaSeconds :type "Float (single-precision)"))
  (bind _blackbricksprite (`self.BlackBrickSprite`))
  (bind _blackbricksprite_2 (`self.BlackBrickSprite`))
  (`/Engine/EditorBlueprintResources/StandardMacros.CompareInt` (`/Game/Blueprint/Background_Sprite.Colour` (`self.BGColour`)) (`self.MyColour`)
    (:`>`
      (`PrimitiveComponent.SetCollisionEnabled` _blackbricksprite_2 "QueryAndPhysics" :!label _label)
      (`SceneComponent.SetVisibility` _blackbricksprite true false))
    (:`==`
      (`PrimitiveComponent.SetCollisionEnabled` _blackbricksprite_2 "NoCollision")
      (`SceneComponent.SetVisibility` _blackbricksprite false false))
    (:`<`
      (goto _label))))

(fn `UserConstructionScript`)