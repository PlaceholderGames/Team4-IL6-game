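; YellowBrick3 is a brick actor that disappears and stops blocking whenever the background's colour matches its own colour index.
; On BeginPlay it caches the first Background_Sprite actor in the level and sets its own colour to a fixed value.
; Every Tick it compares the two colours, hiding the sprite and disabling collision on a match, and restoring both otherwise.
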(event `self.ReceiveBeginPlay`
  (bind _outactors (`GameplayStatics.GetAllActorsOfClass` "/Game/Blueprint/Background_Sprite.Background_Sprite_C"))
  (set `self.BGColour` (`|GetArrayItem` _outactors))
  (set `self.MyColour` 3))

(event `self.ReceiveTick`
  (params (DeltaSeconds :type "Float (single-precision)"))
  (bind _yellowbricksprite (`self.YellowBrickSprite`))
  (bind _yellowbricksprite_2 (`self.YellowBrickSprite`))
  (`/Engine/EditorBlueprintResources/StandardMacros.CompareInt` (`/Game/Blueprint/Background_Sprite.Colour` (`self.BGColour`)) (`self.MyColour`)
    (:`>`
      (`PrimitiveComponent.SetCollisionEnabled` _yellowbricksprite "QueryAndPhysics" :!label _label)
      (`SceneComponent.SetVisibility` _yellowbricksprite_2 true false))
    (:`==`
      (`PrimitiveComponent.SetCollisionEnabled` _yellowbricksprite "NoCollision")
      (`SceneComponent.SetVisibility` _yellowbricksprite_2 false false))
    (:`<`
      (goto _label))))

(fn `UserConstructionScript`)