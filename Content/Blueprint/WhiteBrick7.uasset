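; WhiteBrick7 is a brick actor that disappears and stops colliding while the background shares its colour, index 7.
; On BeginPlay it caches the first Background_Sprite actor in the level and sets its own colour index.
; Every Tick it compares the two values, hiding WhiteBrickSprite and disabling collision on a match, and restoring both otherwise.
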(event `self.ReceiveBeginPlay`
  (bind _outactors (`GameplayStatics.GetAllActorsOfClass` "/Game/Blueprint/Background_Sprite.Background_Sprite_C"))
  (set `self.BGColour` (`|GetArrayItem` _outactors))
  (set `self.MyColour` 7))

(event `self.ReceiveTick`
  (params (DeltaSeconds :type "Float (single-precision)"))
  (bind _whitebricksprite (`self.WhiteBrickSprite`))
  (bind _whitebricksprite_2 (`self.WhiteBrickSprite`))
  (`/Engine/EditorBlueprintResources/StandardMacros.CompareInt` (`/Game/Blueprint/Background_Sprite.Colour` (`self.BGColour`)) (`self.MyColour`)
    (:`>`
      (`PrimitiveComponent.SetCollisionEnabled` _whitebricksprite "QueryAndPhysics" :!label _label)
      (`SceneComponent.SetVisibility` _whitebricksprite_2 true false))
    (:`==`
      (`PrimitiveComponent.SetCollisionEnabled` _whitebricksprite "NoCollision")
      (`SceneComponent.SetVisibility` _whitebricksprite_2 false false))
    (:`<`
      (goto _label))))

(fn `UserConstructionScript`)