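; BlackCrate is a sprite crate that is hidden and passable whenever the background colour matches its own colour.
; On BeginPlay it caches the first Background_Sprite actor and sets its own colour index to 0.
; Each Tick it compares that index with the background's Colour, turning visibility and collision off on a match and on otherwise.
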(event `self.ReceiveBeginPlay`
  (bind _outactors (`GameplayStatics.GetAllActorsOfClass` "/Game/Blueprint/Background_Sprite.Background_Sprite_C"))
  (set `self.BGColour` (`|GetArrayItem` _outactors))
  (set `self.MyColour` 0))

(event `self.ReceiveTick`
  (params (DeltaSeconds :type "Float (single-precision)"))
  (bind _blackcratesprite (`self.BlackCrateSprite`))
  (bind _blackcratesprite_2 (`self.BlackCrateSprite`))
  (`/Engine/EditorBlueprintResources/StandardMacros.CompareInt` (`/Game/Blueprint/Background_Sprite.Colour` (`self.BGColour`)) (`self.MyColour`)
    (:`>`
      (`PrimitiveComponent.SetCollisionEnabled` _blackcratesprite "QueryAndPhysics" :!label _label)
      (`SceneComponent.SetVisibility` _blackcratesprite_2 true false))
    (:`==`
      (`PrimitiveComponent.SetCollisionEnabled` _blackcratesprite "NoCollision")
      (`SceneComponent.SetVisibility` _blackcratesprite_2 false false))
    (:`<`
      (goto _label))))

(fn `UserConstructionScript`)