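; GreenBrick2 is a green brick actor that disappears when the background's colour matches its own.
; On BeginPlay it caches the first Background_Sprite actor and sets its own colour index to green's value.
; Every Tick it compares the two colour indices, turning the sprite's collision and visibility off on a match and on otherwise.
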(event `self.ReceiveBeginPlay`
  (bind _outactors (`GameplayStatics.GetAllActorsOfClass` "/Game/Blueprint/Background_Sprite.Background_Sprite_C"))
  (set `self.BGColour` (`|GetArrayItem` _outactors))
  (set `self.MyColour` 2))

(event `self.ReceiveTick`
  (params (DeltaSeconds :type "Float (single-precision)"))
  (bind _greenbricksprite (`self.GreenBrickSprite`))
  (bind _greenbricksprite_2 (`self.GreenBrickSprite`))
  (`/Engine/EditorBlueprintResources/StandardMacros.CompareInt` (`/Game/Blueprint/Background_Sprite.Colour` (`self.BGColour`)) (`self.MyColour`)
    (:`>`
      (`PrimitiveComponent.SetCollisionEnabled` _greenbricksprite "QueryAndPhysics" :!label _label)
      (`SceneComponent.SetVisibility` _greenbricksprite_2 true false))
    (:`==`
      (`PrimitiveComponent.SetCollisionEnabled` _greenbricksprite "NoCollision")
      (`SceneComponent.SetVisibility` _greenbricksprite_2 false false))
    (:`<`
      (goto _label))))

(fn `UserConstructionScript`)