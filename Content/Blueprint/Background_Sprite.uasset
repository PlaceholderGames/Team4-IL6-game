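; Background sprite Blueprint that cycles its colour through eight values each time the Switching Colours input is released, starting from black.
; The construction script creates a dynamic material instance on the Paper2D sprite, whose BackgroundColour parameter the event graph sets.
; An integer counter wraps from 7 to 0, and repeated divide-by-two remainders turn its three bits into on/off red, green and blue channels.
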(event `self.ReceiveBeginPlay`
  ;[1 1 1] Sets starting colour to black
  (`MaterialInstanceDynamic.SetVectorParameterValue` (`self.DynamicColour`) "BackgroundColour" (`KismetMathLibrary.MakeColor` 0.0)))

(event `InputAction|Switching Colours`
  (params (Key :type "Key Structure" :default "AnyKey"))
  (bind _colour (`self.Colour`))
  (bind (_remainder _returnvalue) (`KismetMathLibrary.FMod` (`KismetMathLibrary.Conv_IntToDouble` (`self.Colour`)) 2.0))
  (bind (_remainder_2 _returnvalue_2) (`KismetMathLibrary.FMod` (`KismetMathLibrary.Conv_IntToDouble` _returnvalue) 2.0))
  ;[1 1 1] Toggles the colour interger from 0 to 7
  (:`Released`
    (set `self.Colour` (+ _colour 1))
    (`/Engine/EditorBlueprintResources/StandardMacros.CompareInt` _colour 7
      (:`>`
        (set `self.Colour` 0))
      (:`==`
        _)
      (:`<`
        _))
    (`MaterialInstanceDynamic.SetVectorParameterValue` (`self.DynamicColour`) "BackgroundColour" (`KismetMathLibrary.MakeColor` _remainder _remainder_2 (`KismetMathLibrary.FMod` (`KismetMathLibrary.Conv_IntToDouble` _returnvalue_2) 2.0) 1.0))))

(fn `UserConstructionScript`
  (bind _returnvalue (`PrimitiveComponent.CreateDynamicMaterialInstance` (`self.PaperSprite`) 0 null))
  (set `self.DynamicColour` _returnvalue))