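; RedBrick1 is a red brick sprite actor that disappears and becomes passable when the background colour matches its own.
; On BeginPlay it caches the first Background_Sprite actor and sets its own colour index to 1.
; Every Tick it compares the background's Colour to that index, disabling collision and visibility on a match and enabling both otherwise.
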(event `self.ReceiveBeginPlay`
  (bind _outactors (`GameplayStatics.GetAllActorsOfClass` "/Game/Blueprint/Background_Sprite.Background_Sprite_C"))
  (set `self.BGColour` (`|GetArrayItem` _outactors))
  (set `self.MyColour` 1))

(event `self.ReceiveTick`
  (params (DeltaSeconds :type "Float (single-precision)"))
  (bind _redbricksprite (`self.RedBrickSprite`))
  (bind _redbricksprite_2 (`self.RedBrickSprite`))
  (`/Engine/EditorBlueprintResources/StandardMacros.CompareInt` (`/Game/Blueprint/Background_Sprite.Colour` (`self.BGColour`)) (`self.MyColour`)
    (:`>`
      (`PrimitiveComponent.SetCollisionEnabled` _redbricksprite_2 "QueryAndPhysics" :!label _label)
      (`SceneComponent.SetVisibility` _redbricksprite true false))
    (:`==`
      (`PrimitiveComponent.SetCollisionEnabled` _redbricksprite_2 "NoCollision")
      (`SceneComponent.SetVisibility` _redbricksprite false false))
    (:`<`
      (goto _label))))

(fn `UserConstructionScript`)