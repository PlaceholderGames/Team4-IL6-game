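; Player character Blueprint with movement along a single axis, jumping and a level reload on death.
; The Move(Right) axis drives movement along world X, while the Jump action starts and stops a hold-sensitive jump tuned in the construction script.
; Being destroyed opens the level named by CurrentLevel.
; The Switching Colours input is a placeholder that only prints a test message.
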(event `InputAxis|Move(Right)`
  (params (AxisValue :type "Float (single-precision)"))
  ;[1 1 1] Movement
  (`self.AddMovementInput` (0.5 0.0 0.0) AxisValue))

(event `InputAction|Jump`
  (params (Key :type "Key Structure" :default "AnyKey"))
  ;[1 1 1] Jumping
  (:`Pressed`
    (`self.Jump`))
  (:`Released`
    (`self.StopJumping`)))

(event `InputAction|Switching Colours`
  (params (Key :type "Key Structure" :default "AnyKey"))
  (:`Released`
    (`KismetSystemLibrary.PrintText` "Hello")))

(event `self.ReceiveDestroyed`
  (`GameplayStatics.OpenLevel` (`self.Current Level`)))

(fn `UserConstructionScript`
  (set `CharacterMovementComponent.JumpZVelocity` 300.0 (`self.CharacterMovement`))
  (set `self.JumpMaxHoldTime` 0.3))